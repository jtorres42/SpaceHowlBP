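; Left-side spawn area trigger that controls whether the side-scroller character (SideScrollerCharacter_Jan) can spawn.
; On Box overlap it hands the character a reference to itself, flags LeftSide, and enables CanSpawn only if SpawnLimitLeft is true.
; Leaving the box clears CanSpawn and LeftSide and sets SpawnLimitLeft back to true.
; All state lives on the character, with the area acting only as a flag setter.
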(event `self.Box.OnComponentBeginOverlap`
  (params (OverlappedComponent :type "PrimitiveComponent Object Reference") (OtherActor :type "Actor Object Reference") (OtherComp :type "PrimitiveComponent Object Reference") (OtherBodyIndex :type Integer) (bFromSweep :type Boolean) (SweepResult :type "HitResult Structure (by ref)"))
  (bind _asside_scroller_character_jan (cast `/Game/SideScrollerBP/Blueprints/SideScrollerCharacter_Jan` OtherActor))
  (set `/Game/SideScrollerBP/Blueprints/SideScrollerCharacter_Jan.SpawnA_Ref` self _asside_scroller_character_jan)
  (set `/Game/SideScrollerBP/Blueprints/SideScrollerCharacter_Jan.LeftSide` true _asside_scroller_character_jan)
  (if (`/Game/SideScrollerBP/Blueprints/SideScrollerCharacter_Jan.SpawnLimitLeft` _asside_scroller_character_jan)
    (set `/Game/SideScrollerBP/Blueprints/SideScrollerCharacter_Jan.CanSpawn` true _asside_scroller_character_jan)))

(event `self.Box.OnComponentEndOverlap`
  (params (OverlappedComponent :type "PrimitiveComponent Object Reference") (OtherActor :type "Actor Object Reference") (OtherComp :type "PrimitiveComponent Object Reference") (OtherBodyIndex :type Integer))
  (bind _asside_scroller_character_jan (cast `/Game/SideScrollerBP/Blueprints/SideScrollerCharacter_Jan` OtherActor))
  (set `/Game/SideScrollerBP/Blueprints/SideScrollerCharacter_Jan.CanSpawn` false _asside_scroller_character_jan)
  (set `/Game/SideScrollerBP/Blueprints/SideScrollerCharacter_Jan.SpawnLimitLeft` true _asside_scroller_character_jan)
  (set `/Game/SideScrollerBP/Blueprints/SideScrollerCharacter_Jan.LeftSide` false _asside_scroller_character_jan))

(fn `UserConstructionScript`)