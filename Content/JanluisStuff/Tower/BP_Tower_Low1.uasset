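; Low-tier defense tower that automatically fires projectiles at AI_Runner enemies, configured from the Tower_Low data table row.
; Sphere overlap assigns targets; without one, Tick runs a throttled sphere trace for the closest runner.
; Tick spawns projectiles carrying target and damage, gated by a fire-rate reload.
; Box overlap halts runners and computes health as the table value minus one, destroying the tower and restoring walking at zero or below.
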(event `NewTarget`
  (bind _returnvalue (`self.K2_GetActorLocation`))
  ;[1 1 1] Searching Target Function
  (set `self.CheckTarget` true)
  (bind (_outhits _returnvalue_2) (`KismetSystemLibrary.SphereTraceMultiForObjects` _returnvalue (- _returnvalue (0.0 0.0 0.0)) (`.Range_14_703DD0104DB7E972EF0A58BB71608086` (break `/Game/JanluisStuff/Tower/TowerStruct` (`self.TowerStruc`))) (`|MakeArray` "ObjectTypeQuery3" :!type "EObjectTypeQuery Enum")))
  (if _returnvalue_2
    (bind _target (`self.Closest Target Calculaton` _outhits))
    (`/Engine/EditorBlueprintResources/StandardMacros.IsValid` _target
      (:`Is Valid`
        (set `self.TowerTarget` _target))
      (:`Is Not Valid`
        _)))
  (`KismetSystemLibrary.Delay` 0.25)
  (set `self.CheckTarget` false))

(event `self.Sphere.OnComponentBeginOverlap`
  (params (OverlappedComponent :type "PrimitiveComponent Object Reference") (OtherActor :type "Actor Object Reference") (OtherComp :type "PrimitiveComponent Object Reference") (OtherBodyIndex :type Integer) (bFromSweep :type Boolean) (SweepResult :type "HitResult Structure (by ref)"))
  ;[1 1 1] Spawn Projectile on Tower
  (`/Engine/EditorBlueprintResources/StandardMacros.IsValid` (`self.TowerTarget`)
    (:`Is Not Valid`
      (bind _asai_runner (cast `/Game/JanluisStuff/AI_Enemy/AI_Runner` OtherActor))
      (set `self.TowerTarget` _asai_runner))))

(event `self.Sphere.OnComponentEndOverlap`
  (params (OverlappedComponent :type "PrimitiveComponent Object Reference") (OtherActor :type "Actor Object Reference") (OtherComp :type "PrimitiveComponent Object Reference") (OtherBodyIndex :type Integer))
  ;[1 1 1] End Overlap/Stop Spawn Projectile
  (if (== (`self.TowerTarget`) OtherActor)
    (set `self.TowerTarget` null)))

(event `self.ReceiveTick`
  (params (DeltaSeconds :type "Float (single-precision)"))
  ;[1 1 1] Shoot to Target & Search New Targets Inside Range
  (`/Engine/EditorBlueprintResources/StandardMacros.IsValid` (`self.TowerTarget`)
    (:`Is Valid`
      (if (not (`self.Reload`))
        (`self.Shoot`)))
    (:`Is Not Valid`
      (if (not (`self.CheckTarget`))
        (`self.NewTarget`)))))

(event `Shoot`
  (bind (_name _damage _range _firerate) (break `/Game/JanluisStuff/Tower/TowerStruct` (`self.TowerStruc`)))
  ;[1 1 1] Shooting to Target
  (set `self.Reload` true)
  (`|SpawnActorFromClass` "/Game/JanluisStuff/Tower/TowerProjectile.TowerProjectile_C" (`self.GetTransform`) "AlwaysSpawn" "OverrideRootScale" null (`self.TowerTarget`) _damage null)
  (`KismetSystemLibrary.Delay` _firerate)
  (set `self.Reload` false))

(event `TowerInit`
  (bind (_name _damage _range _firerate _mesh) (break `/Game/JanluisStuff/Tower/TowerStruct` (`self.TowerStruc`)))
  ;[1 1 1] Towers Meshes
  (`StaticMeshComponent.SetStaticMesh` (`self.TowerMesh`) _mesh)
  (`SphereComponent.SetSphereRadius` (`self.Sphere`) _range true))

(event `self.ReceiveBeginPlay`
  ;[1 1 1] Data Table Tower Selection
  (bind _returnvalue (`|GetDataTableRow` "/Game/JanluisStuff/Tower/TowerDataTable.TowerDataTable" "Tower_Low")
    (:`then`
      (set `self.TowerStruc` _returnvalue)
      (`self.TowerInit`))))

(event `Kill`
  ;[1 1 1] Ai Attack
  (bind _asai_runner (cast `/Game/JanluisStuff/AI_Enemy/AI_Runner` (stale `self.Box.OnComponentBeginOverlap` OtherActor) :!label _label))
  (bind _charactermovement (`Character.CharacterMovement` _asai_runner))
  (`CharacterMovementComponent.DisableMovement` _charactermovement)
  (bind _output_get (set `self.TowerHealth` (- (`.TowerHealth_20_6FC1156B4C142C81562CADAD2E486420` (break `/Game/JanluisStuff/Tower/TowerStruct` (`self.TowerStruc`))) 1.0)))
  (`KismetSystemLibrary.PrintString` (`KismetStringLibrary.Conv_DoubleToString` _output_get))
  (if (<= (`self.TowerHealth`) 0.0)
    (`self.K2_DestroyActor`)
    (`CharacterMovementComponent.SetMovementMode` _charactermovement "MOVE_Walking" 0)))

(event `self.Box.OnComponentBeginOverlap`
  (params (OverlappedComponent :type "PrimitiveComponent Object Reference") (OtherActor :type "Actor Object Reference") (OtherComp :type "PrimitiveComponent Object Reference") (OtherBodyIndex :type Integer) (bFromSweep :type Boolean) (SweepResult :type "HitResult Structure (by ref)"))
  ;[1 1 1] Ai Attack
  (goto _label))

(fn `Closest Target Calculaton`
  (params (HitResults :type "Array of HitResult Structure"))
  (returns (Target :type "/Game/JanluisStuff/AI_Enemy/AI_Runner Object Reference"))
  (locals (TemporaryTarget :type "/Game/JanluisStuff/AI_Enemy/AI_Runner Object Reference") (TempDistance :type "Float (double-precision)" :default 0.0))
  (for _array_element HitResults
    (bind (_bblockinghit _binitialoverlap _time _distance _location _impactpoint _normal _impactnormal _physmat _hitactor) (`GameplayStatics.BreakHitResult` _array_element))
    (bind _asai_runner (cast `/Game/JanluisStuff/AI_Enemy/AI_Runner` _hitactor))
    (`/Engine/EditorBlueprintResources/StandardMacros.IsValid` (`local.TemporaryTarget`)
      (:`Is Valid`
        (bind _returnvalue (`KismetMathLibrary.VSize` (- (`self.K2_GetActorLocation`) (`self.K2_GetActorLocation` _hitactor))))
        (if (< _returnvalue (`local.TempDistance`))
          (set `local.TemporaryTarget` _asai_runner)
          (set `local.TempDistance` _returnvalue)))
      (:`Is Not Valid`
        (set `local.TemporaryTarget` _asai_runner)
        (set `local.TempDistance` _returnvalue))))
  (return (`local.TemporaryTarget`)))

(fn `UserConstructionScript`)