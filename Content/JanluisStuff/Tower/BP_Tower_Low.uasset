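; Defense tower actor that fires projectiles at AI_Runner enemies, with mesh, range, damage, fire rate and health loaded from a data table row.
; It acquires targets through range-box overlaps or a throttled box trace picking the closest runner, then shoots from Tick behind a reload delay.
; Runners touching its inner box start a looping damage timer that destroys it at zero health.
; A separate interaction volume registers the tower with the player character and toggles SpawnLimit.
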(event `NewTarget`
  (bind _returnvalue (`self.K2_GetActorLocation` self))
  ;[1 1 1] Searching Target Function
  (set `self.CheckTarget` true)
  (bind (_outhits _returnvalue_2) (`KismetSystemLibrary.BoxTraceMultiForObjects` _returnvalue (- _returnvalue (0.0 0.0 0.0)) (`.Range_26_703DD0104DB7E972EF0A58BB71608086` (break `/Game/JanluisStuff/Tower/TowerStruct` (`self.TowerStruc`))) (struct) (`|MakeArray` "ObjectTypeQuery3" :!type "EObjectTypeQuery Enum")))
  (if _returnvalue_2
    (bind _target (`self.Closest Target Calculaton` _outhits))
    (`/Engine/EditorBlueprintResources/StandardMacros.IsValid` _target
      (:`Is Valid`
        (set `self.TowerTarget` _target))
      (:`Is Not Valid`
        _)))
  (`KismetSystemLibrary.Delay` 0.25)
  (set `self.CheckTarget` false))

(event `self.DetectEnemy.OnComponentBeginOverlap`
  (params (OverlappedComponent :type "PrimitiveComponent Object Reference") (OtherActor :type "Actor Object Reference") (OtherComp :type "PrimitiveComponent Object Reference") (OtherBodyIndex :type Integer) (bFromSweep :type Boolean) (SweepResult :type "HitResult Structure (by ref)"))
  ;[1 1 1] Spawn Projectile on Tower
  (`/Engine/EditorBlueprintResources/StandardMacros.IsValid` (`self.TowerTarget`)
    (:`Is Not Valid`
      (bind _asai_runner (cast `/Game/JanluisStuff/AI_Enemy/AI_Runner` OtherActor))
      (set `self.TowerTarget` _asai_runner))))

(event `self.DetectEnemy.OnComponentEndOverlap`
  (params (OverlappedComponent :type "PrimitiveComponent Object Reference") (OtherActor :type "Actor Object Reference") (OtherComp :type "PrimitiveComponent Object Reference") (OtherBodyIndex :type Integer))
  ;[1 1 1] End Overlap/Stop Spawn Projectile
  (if (== OtherActor (`self.TowerTarget`))
    (set `self.TowerTarget` null)))

(event `self.ReceiveTick`
  (params (DeltaSeconds :type "Float (single-precision)"))
  ;[1 1 1] Shoot to Target & Search New Targets Inside Range
  (`/Engine/EditorBlueprintResources/StandardMacros.IsValid` (`self.TowerTarget`)
    (:`Is Valid`
      (if (not (`self.Reload`))
        (`self.Shoot`)))
    (:`Is Not Valid`
      (if (not (`self.CheckTarget`))
        (`self.NewTarget`)))))

(event `Shoot`
  (bind (_name _damage _range _firerate) (break `/Game/JanluisStuff/Tower/TowerStruct` (`self.TowerStruc`)))
  ;[1 1 1] Shooting to Target
  (set `self.Reload` true)
  (`|SpawnActorFromClass` "/Game/JanluisStuff/Tower/TowerProjectile.TowerProjectile_C" (`self.GetTransform`) "AlwaysSpawn" "OverrideRootScale" null (`self.TowerTarget`) _damage null)
  (`KismetSystemLibrary.Delay` _firerate)
  (set `self.Reload` false))

(event `TowerInit`
  (bind (_name _damage _range _firerate _mesh) (break `/Game/JanluisStuff/Tower/TowerStruct` (`self.TowerStruc`)))
  ;[1 1 1] Towers Meshes
  (`StaticMeshComponent.SetStaticMesh` (`self.TowerMesh`) _mesh)
  (`BoxComponent.SetBoxExtent` (`self.DetectEnemy`) _range true))

(event `self.ReceiveBeginPlay`
  ;[1 1 1] Data Table Tower Selection
  (bind _returnvalue (`|GetDataTableRow` "/Game/JanluisStuff/Tower/TowerDataTable.TowerDataTable" (`self.TowerNames`))
    (:`then`
      (set `self.TowerStruc` _returnvalue)
      (`self.TowerInit`)
      (set `self.TowerHealth` (`.TowerHealth_20_6FC1156B4C142C81562CADAD2E486420` (break `/Game/JanluisStuff/Tower/TowerStruct` (`self.TowerStruc`)))))))

(event `StopLoop`
  ;[1 1 1] Ai Attack
  (`KismetSystemLibrary.K2_ClearTimer` null "DamageTower")
  (`self.K2_DestroyActor`)
  (set `self.CheckLoop` false))

(event `self.Box.OnComponentBeginOverlap`
  (params (OverlappedComponent :type "PrimitiveComponent Object Reference") (OtherActor :type "Actor Object Reference") (OtherComp :type "PrimitiveComponent Object Reference") (OtherBodyIndex :type Integer) (bFromSweep :type Boolean) (SweepResult :type "HitResult Structure (by ref)"))
  ;[1 1 1] Ai Attack
  (bind _asai_runner (cast `/Game/JanluisStuff/AI_Enemy/AI_Runner` OtherActor))
  (set `/Game/JanluisStuff/AI_Enemy/AI_Runner.Tower_Low` self _asai_runner)
  (`/Game/JanluisStuff/AI_Enemy/AI_Runner.ItsOn` _asai_runner)
  (set `self.CheckLoop` true)
  (`KismetSystemLibrary.K2_SetTimer` null "DamageTower" 0.5 (`self.CheckLoop`)))

(event `self.Box.OnComponentEndOverlap`
  (params (OverlappedComponent :type "PrimitiveComponent Object Reference") (OtherActor :type "Actor Object Reference") (OtherComp :type "PrimitiveComponent Object Reference") (OtherBodyIndex :type Integer))
  ;[1 1 1] Ai Attack
  (cast `/Game/JanluisStuff/AI_Enemy/AI_Runner` OtherActor)
  (`KismetSystemLibrary.K2_ClearTimer` null "DamageTower")
  (set `self.CheckLoop` false))

(event `self.CharacInteraction.OnComponentBeginOverlap`
  (params (OverlappedComponent :type "PrimitiveComponent Object Reference") (OtherActor :type "Actor Object Reference") (OtherComp :type "PrimitiveComponent Object Reference") (OtherBodyIndex :type Integer) (bFromSweep :type Boolean) (SweepResult :type "HitResult Structure (by ref)"))
  ;[1 1 1] Character Spawn Tower
  (bind _asside_scroller_character_jan (cast `/Game/SideScrollerBP/Blueprints/SideScrollerCharacter_Jan` OtherActor))
  (set `/Game/SideScrollerBP/Blueprints/SideScrollerCharacter_Jan.TowersRef` self _asside_scroller_character_jan)
  (set `self.Destroy` true)
  (set `/Game/SideScrollerBP/Blueprints/SideScrollerCharacter_Jan.SpawnLimit` false _asside_scroller_character_jan))

(event `self.CharacInteraction.OnComponentEndOverlap`
  (params (OverlappedComponent :type "PrimitiveComponent Object Reference") (OtherActor :type "Actor Object Reference") (OtherComp :type "PrimitiveComponent Object Reference") (OtherBodyIndex :type Integer))
  ;[1 1 1] Character Spawn Tower
  (bind _asside_scroller_character_jan (cast `/Game/SideScrollerBP/Blueprints/SideScrollerCharacter_Jan` OtherActor))
  (set `self.Destroy` false)
  (set `/Game/SideScrollerBP/Blueprints/SideScrollerCharacter_Jan.SpawnLimit` true _asside_scroller_character_jan))

(fn `Closest Target Calculaton`
  (params (HitResults :type "Array of HitResult Structure"))
  (returns (Target :type "/Game/JanluisStuff/AI_Enemy/AI_Runner Object Reference"))
  (locals (TemporaryTarget :type "/Game/JanluisStuff/AI_Enemy/AI_Runner Object Reference") (TempDistance :type "Float (double-precision)" :default 0.0))
  (for _array_element HitResults
    (bind (_bblockinghit _binitialoverlap _time _distance _location _impactpoint _normal _impactnormal _physmat _hitactor) (`GameplayStatics.BreakHitResult` _array_element))
    (bind _asai_runner (cast `/Game/JanluisStuff/AI_Enemy/AI_Runner` _hitactor))
    (`/Engine/EditorBlueprintResources/StandardMacros.IsValid` (`local.TemporaryTarget`)
      (:`Is Valid`
        (bind _returnvalue (`KismetMathLibrary.VSize` (- (`self.K2_GetActorLocation`) (`self.K2_GetActorLocation` _hitactor))))
        (if (< _returnvalue (`local.TempDistance`))
          (set `local.TemporaryTarget` _asai_runner)
          (set `local.TempDistance` _returnvalue)))
      (:`Is Not Valid`
        (set `local.TemporaryTarget` _asai_runner)
        (set `local.TempDistance` _returnvalue))))
  (return (`local.TemporaryTarget`)))

(fn `DamageTower`
  (bind _output_get (set `self.TowerHealth` (- (`self.TowerHealth`) 1.0)))
  (`KismetSystemLibrary.PrintString` (`KismetStringLibrary.Conv_DoubleToString` _output_get))
  (if (<= (`self.TowerHealth`) 0.0)
    (`/Game/JanluisStuff/AI_Enemy/AI_Runner.TurnOff` (`self.TowerTarget`))
    (`self.StopLoop`)))

(fn `UserConstructionScript`)