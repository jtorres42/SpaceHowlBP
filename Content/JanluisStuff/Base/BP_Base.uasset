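; BP_Base is a base with health that AI_Runner enemies drain, ending in game over at zero.
; A runner overlapping the box receives a base reference and an ItsOn call, then a looping timer runs DamageBase until an overlap end clears it.
; At zero health, DamageBase calls TurnOff on AirunnerRef, which is not assigned here, and StopLoop shows the game-over HUD, then the main menu after a delay.
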(event `self.Box.OnComponentBeginOverlap`
  (params (OverlappedComponent :type "PrimitiveComponent Object Reference") (OtherActor :type "Actor Object Reference") (OtherComp :type "PrimitiveComponent Object Reference") (OtherBodyIndex :type Integer) (bFromSweep :type Boolean) (SweepResult :type "HitResult Structure (by ref)"))
  (bind _asai_runner (cast `/Game/JanluisStuff/AI_Enemy/AI_Runner` OtherActor))
  (set `/Game/JanluisStuff/AI_Enemy/AI_Runner.BaseRef` self _asai_runner)
  (set `self.CheckLoop` true)
  (`/Game/JanluisStuff/AI_Enemy/AI_Runner.ItsOn` _asai_runner)
  (`KismetSystemLibrary.K2_SetTimer` null "DamageBase" 0.5 (`self.CheckLoop`)))

(event `self.Box.OnComponentEndOverlap`
  (params (OverlappedComponent :type "PrimitiveComponent Object Reference") (OtherActor :type "Actor Object Reference") (OtherComp :type "PrimitiveComponent Object Reference") (OtherBodyIndex :type Integer))
  (cast `/Game/JanluisStuff/AI_Enemy/AI_Runner` OtherActor)
  (`KismetSystemLibrary.K2_ClearTimer` null "DamageBase")
  (set `self.CheckLoop` false))

(event `StopLoop`
  (bind _returnvalue (`GameplayStatics.GetPlayerController` 0))
  (`KismetSystemLibrary.K2_ClearTimer` null "DamageBase")
  (set `self.CheckLoop` false)
  (bind _returnvalue_2 (`|CreateWidget` "/Game/JanluisStuff/Base/HUD_GameOver.HUD_GameOver_C" _returnvalue))
  (`UserWidget.AddToViewport` _returnvalue_2 0)
  (`KismetSystemLibrary.Delay` 3.0)
  (bind _returnvalue_3 (`|CreateWidget` "/Game/JaphetStuff/MainMenu_BP.MainMenu_BP_C" _returnvalue))
  (`UserWidget.AddToViewport` _returnvalue_3 0))

(fn `DamageBase`
  (bind _output_get (set `self.BaseHealth` (- (`self.BaseHealth`) 1.0)))
  (`KismetSystemLibrary.PrintString` (`KismetStringLibrary.Conv_DoubleToString` _output_get))
  (if (<= (`self.BaseHealth`) 0.0)
    (`/Game/JanluisStuff/AI_Enemy/AI_Runner.TurnOff` (`self.AirunnerRef`))
    (`self.StopLoop`)))

(fn `UserConstructionScript`)